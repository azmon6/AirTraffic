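; Game mode for an air traffic game that sets up the map's air points and a command-line UI.
; At BeginPlay it spawns named markers from RevisionTWO table coordinates scaled to the map, and measures the UTEKA–AMTOV reference distance.
; Helpers generate random plane names, attach info actors to planes and forward text to input processing.
; Pausing toggles plane ticking, with IsGamePaused counterintuitively true while planes run.
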(event EventBeginPlay
  (CallFunction|AddingAirPoints)
  (bind _returnvalue (UserInterface|CreateWidget "/Game/UI/CommandLineUI.CommandLineUI_C" (Game|GetPlayerController 0)))
  (UserInterface|Viewport|AddtoViewport _returnvalue 0)
  (CallFunction|CalculateDistAmUt)
  (Variables|Default|SetIsGamePaused true))

(event EventChangeCommandLineBool
  (Variables|Default|SetbCommandLine false)
  (Variables|Default|SetCommandLineText ""))

(event EventAddInfotoPlane
  (params (Arg :type Plane%20Actor%20Object%20Reference))
  (bind _returnvalue (Game|SpawnActorfromClass "/Game/Blueprint/PlaneInfoBP.PlaneInfoBP_C" (Math|Conversions|ToTransform(Vector) (- (Transformation|GetActorLocation Arg) "10.000000,10.000000,-20.000000")) "AlwaysSpawn" 0 0))
  (bind _asplane_actor_bp (Utilities|Casting|CastToPlaneActorBP Arg)
    (:then
      (Variables|/Game/Blueprint/PlaneInfoBP.PlaneInfoBP_C|SetPlaneDesignated _returnvalue _asplane_actor_bp))
    (:CastFailed
      (Development|PrintString "Hello2"))))

(event EventPauseAirplanes
  (bind _output_get (Variables|Default|SetIsGamePaused (not (Variables|Default|GetIsGamePaused))))
  (for _array_element (Variables|Default|GetPlanesRef)
    (Actor|Tick|SetActorTickEnabled _array_element _output_get)))

(fn ConstructionScript)

(fn GetAirPointLoc
  (params (Arg :type String))
  (bind _map (Variables|Default|GetMap))
  (bind _returnvalue (Transformation|GetActorTransform _map))
  (bind (_location _rotation _scale) (Math|Transform|BreakTransform _returnvalue))
  (bind (_x _y _z) (Math|Vector|BreakVector _location))
  (bind (_x_2 _y_2) (Math|Vector|BreakVector _scale))
  (bind _returnvalue_2 (Utilities|GetDataTableRow "/Game/Data/RevisionTWO.RevisionTWO" (Utilities|String|StringToName Arg))
    (:then
      (return (Math|Conversions|ToTransform(Vector) (Math|Vector|MakeVector (+ _x (* _x_2 (.X (Utilities|Struct|BreakAirPointStruct _returnvalue_2)))) (+ _y (* _y_2 (.Y (Utilities|Struct|BreakAirPointStruct _returnvalue_2)))) (+ _z 4.0)))))
    (:RowNotFound
      (return (Math|Transform|MakeTransform "0, 0, 0")))))

(fn GetRandomPlaneName
  (bind _returnvalue (Utilities|GetDataTableRow "/Game/Data/AirNames.AirNames" (Utilities|String|StringToName (Utilities|String|ToString(Integer) (Math|Random|RandomIntegerinRange 0 100))))
    (:then
      (return (Utilities|String|Append (Utilities|Struct|BreakAirNameStruct _returnvalue) (Utilities|String|ToString(Integer) (Math|Random|RandomIntegerinRange 1000 9999)))))
    (:RowNotFound
      (Development|PrintString "RowNotFound")
      (return "FAIL"))))

(fn AddingAirPoints
  (bind _outactors (Actor|GetAllActorsOfClass "/Game/Blueprint/MapBP.MapBP_C"))
  (for _array_element _outactors
    (Variables|Default|SetMap _array_element)
    (bind _outrownames (DataTable|GetDataTableRowNames "/Game/Data/RevisionTWO.RevisionTWO"))
    (for _array_element_2 _outrownames
      (bind _returnvalue (Utilities|GetDataTableRow "/Game/Data/RevisionTWO.RevisionTWO" _array_element_2)
        (:then
          (bind _returnvalue_2 (Game|SpawnActorfromClass "/Game/Blueprint/TestingSpriteBP.TestingSpriteBP_C" (Math|Conversions|ToTransform(Vector) (Math|Vector|MakeVector (+ (.X (Math|Vector|BreakVector (.Location (Math|Transform|BreakTransform (Transformation|GetActorTransform (Variables|Default|GetMap)))))) (* (.X (Math|Vector|BreakVector (.Scale (Math|Transform|BreakTransform (Transformation|GetActorTransform (Variables|Default|GetMap)))))) (.X (Utilities|Struct|BreakAirPointStruct _returnvalue)))) (+ (.Y (Math|Vector|BreakVector (.Location (Math|Transform|BreakTransform (Transformation|GetActorTransform (Variables|Default|GetMap)))))) (* (.Y (Math|Vector|BreakVector (.Scale (Math|Transform|BreakTransform (Transformation|GetActorTransform (Variables|Default|GetMap)))))) (.Y (Utilities|Struct|BreakAirPointStruct _returnvalue)))) (+ (.Z (Math|Vector|BreakVector (.Location (Math|Transform|BreakTransform (Transformation|GetActorTransform (Variables|Default|GetMap)))))) 3.0))) "AlwaysSpawn" 0 0))
          (Transformation|SetActorScale3D _returnvalue_2 "2.000000, 0,2.000000")
          (Default|SetName _returnvalue_2 (Utilities|String|ToString(Name) _array_element_2)))))))

(fn TestingUMG
  (params (Input :type String))
  (Class|AirTrafficGameMode|InputProcessing Input))

(fn CalculateDistAmUt
  (bind _returnvalue (CallFunction|GetAirPointLoc "UTEKA"))
  (bind _returnvalue_2 (CallFunction|GetAirPointLoc "AMTOV"))
  (Variables|Default|SetDistInGameAmtovUteka (Math|Vector|VectorLength (- (.Location (Math|Transform|BreakTransform _returnvalue_2)) (.Location (Math|Transform|BreakTransform _returnvalue))))))