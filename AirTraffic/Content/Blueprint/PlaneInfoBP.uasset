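; Floating info tag actor that follows a designated plane and shows its name, flight level and speed in a PlaneInfoUI widget.
; Each tick it sits at a stored offset from the plane, refreshes the text and has the plane draw debug lines between them.
; Clicked toggles cursor-trace dragging and saves the new offset on release.
; It destroys itself once the plane is invalid.
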(event EventBeginPlay
  (Rendering|SetVisibility (Variables|Default|GetPlane) false false)
  (Variables|Default|SetIsClicked false)
  (Variables|Default|SetDistance "100.000000,100.000000, 0"))

(event EventTick
  (params (DeltaSeconds :type Float%20%28single-precision%29))
  (bind _planedesignated (Variables|Default|GetPlaneDesignated))
  (Utilities|IsValid (Variables|Default|GetPlaneDesignated)
    (:Is%20Valid
      (if (Variables|Default|GetIsClicked)
        (Transformation|SetActorLocation (.Location (Collision|BreakHitResult (.HitResult (Game|Player|GetHitResultUnderCursorbyChannel (Game|GetPlayerController 0) "TraceTypeQuery1" true)))) false false)
        (else
          (Transformation|SetActorLocation (+ (- (Transformation|GetActorLocation (Variables|Default|GetPlaneDesignated)) (* (Variables|Default|GetDistance) -1.0)) "0, 0,10.000000") false false)))
      (bind (_name _flightlevel _speed) (Class|PlaneActor|GiveInfo (Variables|Default|GetPlaneDesignated)))
      (bind _asplane_info_ui (Utilities|Casting|CastToPlaneInfoUI (UserInterface|GetUserWidgetObject (Variables|Default|GetInfo))))
      (Default|ChangeText _asplane_info_ui (Utilities|String|Append _name " 
" (Utilities|String|ToString(Integer) (Math|Float|Round _flightlevel)) " 
" (Utilities|String|ToString(Float) _speed)))
      (Class|PlaneActor|DrawDebugLines _planedesignated (Transformation|GetActorLocation) (Transformation|GetActorLocation _planedesignated)))
    (:Is%20Not%20Valid
      (Actor|DestroyActor))))

(fn ConstructionScript)

(fn Clicked
  (if (Variables|Default|GetIsClicked)
    (Variables|Default|SetDistance (- (Transformation|GetActorLocation) (Transformation|GetActorLocation (Variables|Default|GetPlaneDesignated)))))
  (Variables|Default|SetIsClicked (not (Variables|Default|GetIsClicked))))