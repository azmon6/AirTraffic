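; Plane Blueprint with a toggleable trajectory display that starts hidden.
; Each tick it calls DrawTrajectory while the flag is on, and otherwise deactivates the Beam particle component.
; A helper derives a destination point from a center, rotation and distance, adding the distance to the forward vector rather than scaling it.
; The beam activation and endpoint-setting nodes in the event graph are unconnected.
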(event EventBeginPlay
  (Variables|Default|SetbShowTrajectory false))

(event EventTick
  (params (DeltaSeconds :type Float%20%28single-precision%29))
  (if (Variables|Default|GetbShowTrajectory)
    (Class|PlaneActor|DrawTrajectory)
    (else
      (Components|Activation|Deactivate (Variables|Default|GetBeam)))))

(fn ConstructionScript)

(fn GetNewRotatedDestPoint
  (params (Center :type Vector%20%28by%20ref%29 :default "0, 0, 0") (Rotation :type Rotator%20%28by%20ref%29 :default "0, 0, 0") (Distance :type Float%20%28single-precision%29%20%28by%20ref%29))
  (return (+ Center (+ (Math|Vector|GetForwardVector Rotation) Distance))))

(fn ShowTrajectory
  (Variables|Default|SetbShowTrajectory (not (Variables|Default|GetbShowTrajectory))))