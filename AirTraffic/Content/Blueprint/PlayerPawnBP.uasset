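; PlayerPawnBP is the player pawn, providing free movement in three dimensions relative to its camera's orientation.
; Three input axes (MoveUpDown, MoveLeftRight, MoveInOut) each feed AddMovementInput along the camera's world-space up, right or forward vector.
; Because directions come from the full camera rotation, any pitch or roll also tilts the movement axes.
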(event Input|AxisEvents|InputAxisMoveUpDown
  (params (AxisValue :type Float%20%28single-precision%29))
  (Pawn|Input|AddMovementInput (Math|Vector|GetUpVector (Transformation|GetWorldRotation (Variables|Default|GetCamera))) AxisValue false))

(event Input|AxisEvents|InputAxisMoveLeftRight
  (params (AxisValue :type Float%20%28single-precision%29))
  (Pawn|Input|AddMovementInput (Math|Vector|GetRightVector (Transformation|GetWorldRotation (Variables|Default|GetCamera))) AxisValue false))

(event Input|AxisEvents|InputAxisMoveInOut
  (params (AxisValue :type Float%20%28single-precision%29))
  (Pawn|Input|AddMovementInput (Math|Vector|GetForwardVector (Transformation|GetWorldRotation (Variables|Default|GetCamera))) AxisValue false))

(fn ConstructionScript)