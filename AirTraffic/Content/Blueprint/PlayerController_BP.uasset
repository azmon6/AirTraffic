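; Player controller for an air traffic game that shows the mouse cursor and handles clicking, pausing and the command line.
; Its construction script caches the AirTrafficGameModeBP, which receives the command line flag and the pause-airplanes call.
; Both click press and release trace under the cursor for Pawn and Vehicle objects, calling Clicked on plane info actors or ShowTrajectory on plane actors.
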(event EventBeginPlay
  (Variables|Default|SetbShowMouseCursor true))

(event Input|ActionEvents|InputActionPauseGame
  (params (Key :type Key%20Structure))
  (:Released
    (Class|AirTrafficGameMode|PauseAirplanes (Variables|Default|GetGameMode))))

(event Input|ActionEvents|InputActionOpenCommandLine
  (params (Key :type Key%20Structure))
  (:Released
    (Variables|/Game/Blueprint/AirTrafficGameModeBP.AirTrafficGameModeBP_C|SetbCommandLine (Variables|Default|GetGameMode) true)))

(event Input|ActionEvents|InputActionClick
  (params (Key :type Key%20Structure))
  (bind _returnvalue (Game|GetPlayerController 0))
  (bind _array (Utilities|Array|MakeArray "ObjectTypeQuery3" "ObjectTypeQuery5"))
  (bind (_hitresult _returnvalue_2) (Class|PlayerController|GetHitResultUnderCursorforObjects _returnvalue _array true))
  (bind _hitactor (Collision|BreakHitResult _hitresult))
  (:Pressed
    (if _returnvalue_2 :!label _label
      (bind _asplane_info_bp (Utilities|Casting|CastToPlaneInfoBP _hitactor)
        (:then
          (Default|Clicked _asplane_info_bp))
        (:CastFailed
          (bind _asplane_actor_bp (Utilities|Casting|CastToPlaneActorBP _hitactor))
          (Default|ShowTrajectory _asplane_actor_bp)))))
  (:Released
    (goto _label)))

(fn ConstructionScript
  (bind _asair_traffic_game_mode_bp (Utilities|Casting|CastToAirTrafficGameModeBP (Game|GetGameMode)))
  (Variables|Default|SetGameMode _asair_traffic_game_mode_bp))